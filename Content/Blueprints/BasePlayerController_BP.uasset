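; Base player controller for a first-person spellcasting game, handling movement, jump, look, HUD creation and quit on Escape.
; On possession it spawns the first SpellList spell at the pawn's casting point, and fire inputs start and end its primary and alternate casts.
; The NextSpell axis wraps through SpellList, replacing the spell actor and updating the HUD.
; Holding P and G unlocks a hidden firebolt shotgun spell via a Tick check.
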(event EventTick
  (params (DeltaSeconds :type Float%20%28single-precision%29))
  (bind _array_element (Utilities|Array|ForEachLoopwithBreak (Variables|Default|GetSpellList) :!label _label)
    (:LoopBody
      (if (== _array_element "/Game/Blueprints/Spells/ProjectileSpells/FireboltShotgunSpell_BP.FireboltShotgunSpell_BP_C")
        (goto _label Break)))
    (:Completed
      (if (not (== _array_element "/Game/Blueprints/Spells/ProjectileSpells/FireboltShotgunSpell_BP.FireboltShotgunSpell_BP_C"))
        (if (Variables|Default|GetP_KeyPressed)
          (if (Variables|Default|GetG_KeyPressed)
            (Utilities|Array|Add (Variables|Default|GetSpellList) "/Game/Blueprints/Spells/ProjectileSpells/FireboltShotgunSpell_BP.FireboltShotgunSpell_BP_C")))))))

(event EventBeginPlay
  (bind _currentspell (Variables|Default|GetCurrentSpell))
  (bind _returnvalue (UserInterface|CreateWidget "/Game/Blueprints/Widgets/HUDWidget_BP.HUDWidget_BP_C" self))
  (bind _output_get (Variables|Default|SetHUD%20Widget _returnvalue))
  (UserInterface|Viewport|AddtoViewport _output_get 0)
  (Variables|/Game/Blueprints/Widgets/HUDWidget_BP.HUDWidget_BP_C|SetSpellSelectedText (Variables|Default|GetHUD%20Widget) (Variables|/Game/Blueprints/Spells/BaseSpell_BP.BaseSpell_BP_C|GetSpell%20Name _currentspell))
  (bind _asbase_player_pawn_bp (Utilities|Casting|CastToBasePlayerPawn_BP (Pawn|GetControlledPawn)))
  (Variables|/Game/Blueprints/Spells/BaseSpell_BP.BaseSpell_BP_C|SetCasterPawn _currentspell _asbase_player_pawn_bp)
  (Variables|Default|SetbShowMouseCursor false))

(event EventPossess
  (params (PossessedPawn :type Pawn%20Object%20Reference))
  (bind _asbase_player_pawn_bp (Utilities|Casting|CastToBasePlayerPawn_BP PossessedPawn))
  (bind _returnvalue (Game|SpawnActorfromClass (Utilities|Array|Get(acopy) (Variables|Default|GetSpellList)) (Transformation|GetWorldTransform (Variables|/Game/Blueprints/BasePlayerPawn_BP.BasePlayerPawn_BP_C|GetFirstPersonCamera _asbase_player_pawn_bp)) "Undefined" PossessedPawn PossessedPawn))
  (Transformation|AttachComponentToComponent _returnvalue (Variables|/Game/Blueprints/BasePlayerPawn_BP.BasePlayerPawn_BP_C|GetSpellCastingPoint _asbase_player_pawn_bp) "None" "SnapToTarget" "SnapToTarget" "SnapToTarget" true)
  (Variables|Default|SetCurrentSpell _returnvalue))

(event Input|ActionEvents|InputActionFire
  (params (Key :type Key%20Structure :default "None"))
  (bind _currentspell (Variables|Default|GetCurrentSpell))
  (:Pressed
    (Default|CastSpell _currentspell))
  (:Released
    (Default|EndCastSpell _currentspell)))

(event Input|ActionEvents|InputActionSecondaryFire
  (params (Key :type Key%20Structure :default "None"))
  (bind _currentspell (Variables|Default|GetCurrentSpell))
  (:Pressed
    (Default|AltCastSpell _currentspell))
  (:Released
    (Default|AltEndCastSpell _currentspell)))

(event Input|AxisEvents|InputAxisNextSpell
  (params (AxisValue :type Float%20%28single-precision%29))
  (bind _returnvalue (Math|Float|Clamp(Float) AxisValue -1.0))
  (bind _returnvalue_2 (Math|Float|Truncate _returnvalue))
  ;[1 1 1] Checks if axis is not equal to 0.
  (if (!= _returnvalue 0.0)
    (if (> (+ _returnvalue_2 (Variables|Default|GetSpellCursor)) (- (Utilities|Array|Length (Variables|Default|GetSpellList)) 1))
      (Variables|Default|SetSpellCursor (- (+ (Variables|Default|GetSpellCursor) _returnvalue_2) (Utilities|Array|Length (Variables|Default|GetSpellList))))
      (elif (< (+ _returnvalue_2 (Variables|Default|GetSpellCursor)) 0)
        (Variables|Default|SetSpellCursor (+ (Variables|Default|GetSpellCursor) _returnvalue_2 (Utilities|Array|Length (Variables|Default|GetSpellList))))
        (else
          (Variables|Default|SetSpellCursor (+ (Variables|Default|GetSpellCursor) _returnvalue_2)))))
    (bind _asbase_player_pawn_bp (Utilities|Casting|CastToBasePlayerPawn_BP (Pawn|GetControlledPawn))
      (:then
        (bind _returnvalue_3 (Game|SpawnActorfromClass (Utilities|Array|Get(acopy) (Variables|Default|GetSpellList) (Variables|Default|GetSpellCursor)) (Math|Transform|MakeTransform "0, 0, 0" "0, 0, 0" "1,1,1") "Undefined" _asbase_player_pawn_bp _asbase_player_pawn_bp))
        (Transformation|AttachComponentToComponent _returnvalue_3 (Variables|/Game/Blueprints/BasePlayerPawn_BP.BasePlayerPawn_BP_C|GetSpellCastingPoint _asbase_player_pawn_bp) "None" "SnapToTarget" "SnapToTarget" "SnapToTarget" true)
        (Actor|DestroyActor (Variables|Default|GetCurrentSpell))
        (bind _output_get (Variables|Default|SetCurrentSpell _returnvalue_3))
        (Variables|/Game/Blueprints/Widgets/HUDWidget_BP.HUDWidget_BP_C|SetSpellSelectedText (Variables|Default|GetHUD%20Widget) (Variables|/Game/Blueprints/Spells/BaseSpell_BP.BaseSpell_BP_C|GetSpell%20Name _output_get))
        (bind _asbase_player_pawn_bp_2 (Utilities|Casting|CastToBasePlayerPawn_BP (Pawn|GetControlledPawn)))
        (Variables|/Game/Blueprints/Spells/BaseSpell_BP.BaseSpell_BP_C|SetCasterPawn _output_get _asbase_player_pawn_bp_2))
      (:CastFailed
        (Development|PrintString "Failed to cast" true true "(R=1.000000,G=0.076232,B=0.000000,A=1.000000)")))))

(event Input|KeyboardEvents|P
  (params (Key :type Key%20Structure :default "None"))
  (:Pressed
    (Variables|Default|SetP_KeyPressed true))
  (:Released
    (Variables|Default|SetP_KeyPressed false)))

(event Input|KeyboardEvents|G
  (params (Key :type Key%20Structure :default "None"))
  (:Pressed
    (Variables|Default|SetG_KeyPressed true))
  (:Released
    (Variables|Default|SetG_KeyPressed false)))

(event Input|KeyboardEvents|Escape
  (params (Key :type Key%20Structure :default "None"))
  (:Pressed
    (Game|QuitGame 0 "Quit" false)))

(event Input|ActionEvents|InputActionJump
  (params (Key :type Key%20Structure))
  (bind _returnvalue (Pawn|GetControlledPawn))
  ;[1 1 1] Movement controls.
  ;;[1 1 1] Handles jumping.
  (:Pressed
    (bind _ascharacter (Utilities|Casting|CastToCharacter _returnvalue))
    (Character|Jump _ascharacter))
  (:Released
    (bind _ascharacter_2 (Utilities|Casting|CastToCharacter _returnvalue))
    (Character|StopJumping _ascharacter_2)))

(event Input|AxisEvents|InputAxisMoveForward
  (params (AxisValue :type Float%20%28single-precision%29))
  (bind _returnvalue (Pawn|GetControlledPawn))
  ;[1 1 1] Movement controls.
  ;;[1 1 1] Handles moving forward and backwards.
  (Pawn|Input|AddMovementInput _returnvalue (Transformation|GetActorForwardVector _returnvalue) AxisValue false))

(event Input|AxisEvents|InputAxisStrafeRight
  (params (AxisValue :type Float%20%28single-precision%29))
  (bind _returnvalue (Pawn|GetControlledPawn))
  ;[1 1 1] Movement controls.
  ;;[1 1 1] Handles moving left and right.
  (Pawn|Input|AddMovementInput _returnvalue (Transformation|GetActorRightVector _returnvalue) AxisValue false))

(event Input|AxisEvents|InputAxisTurn
  (params (AxisValue :type Float%20%28single-precision%29))
  ;[1 1 1] Camera controls.
  (Pawn|Input|AddControllerYawInput (Pawn|GetControlledPawn) AxisValue))

(event Input|AxisEvents|InputAxisLookUp
  (params (AxisValue :type Float%20%28single-precision%29))
  ;[1 1 1] Camera controls.
  (Pawn|Input|AddControllerPitchInput (Pawn|GetControlledPawn) AxisValue))

(fn ConstructionScript)