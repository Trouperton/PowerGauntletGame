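; Projectile spell Blueprint for a firebolt shotgun, firing a randomly sized burst of projectiles in a spread.
; CastSpell runs the parent cast logic, then loops a random number of times, up to about a hundred, spawning the Projectile class at the spell actor's location.
; Each spawn keeps the actor's roll and randomly offsets pitch and yaw within ten degrees either way.
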(event EventCastSpell
  (bind _self self)
  (bind _returnvalue (Transformation|GetActorTransform _self))
  (bind (_location _rotation) (Math|Transform|BreakTransform _returnvalue))
  (bind (_roll _pitch _yaw) (Math|Rotator|BreakRotator _rotation))
  (|CallParentFunction)
  (for _index (range 0 (Math|Random|RandomInteger 100))
    (Game|SpawnActorfromClass (Variables|Default|GetProjectile) (Math|Transform|MakeTransform _location (Math|Rotator|MakeRotator _roll (+ _pitch (Math|Random|RandomFloatinRange -1e+01 1e+01)) (+ _yaw (Math|Random|RandomFloatinRange -1e+01 1e+01))) (Math|Vector|MakeVector 1.0 1.0 1.0)) "Undefined" 0 0)))

(fn ConstructionScript
  (|CallParentFunction))