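; Brazier level asset that can be lit or extinguished by elemental spell projectiles.
; On BeginPlay it applies its IsLit state through Light or Extinguish, which toggle the Fire component and point light visibility and update the flag.
; When a BaseSpellProjectile_BP hits it, the projectile's ElementType is compared to the IgnitingElement and ExtinguishingElement to choose which function runs.
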(event EventBeginPlay
  (if (Variables|Default|GetIsLit)
    (CallFunction|Light)
    (else
      (CallFunction|Extinguish))))

(event Collision|EventActorBeginOverlap
  (params (OtherActor :type Actor%20Object%20Reference)))

(event EventTick
  (params (DeltaSeconds :type Float%20%28single-precision%29)))

(event Collision|EventHit
  (params (MyComp :type Primitive%20Component%20Object%20Reference) (Other :type Actor%20Object%20Reference) (OtherComp :type Primitive%20Component%20Object%20Reference) (bSelfMoved :type Boolean) (HitLocation :type Vector :default "0, 0, 0") (HitNormal :type Vector :default "0, 0, 0") (NormalImpulse :type Vector :default "0, 0, 0") (Hit :type Hit%20Result%20Structure%20%28by%20ref%29))
  (bind _asbase_spell_projectile_bp (Utilities|Casting|CastToBaseSpellProjectile_BP Other))
  (if (== (Variables|/Game/Blueprints/Spells/ProjectileSpells/SpellProjectiles/BaseSpellProjectile_BP.BaseSpellProjectile_BP_C|GetElementType _asbase_spell_projectile_bp) (Variables|Default|GetIgnitingElement))
    (CallFunction|Light)
    (elif (== (Variables|/Game/Blueprints/Spells/ProjectileSpells/SpellProjectiles/BaseSpellProjectile_BP.BaseSpellProjectile_BP_C|GetElementType _asbase_spell_projectile_bp) (Variables|Default|GetExtinguishingElement))
      (CallFunction|Extinguish))))

(fn ConstructionScript)

(fn Light
  (Components|Activation|Activate (Variables|Default|GetFire) false)
  (Rendering|SetVisibility (Variables|Default|GetFirePointLight) true false)
  (Variables|Default|SetIsLit true))

(fn Extinguish
  (Components|Activation|Deactivate (Variables|Default|GetFire))
  (Rendering|SetVisibility (Variables|Default|GetFirePointLight) false false)
  (Variables|Default|SetIsLit false))