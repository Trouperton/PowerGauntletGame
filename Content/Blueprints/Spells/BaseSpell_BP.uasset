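; Base spell actor Blueprint that defines cast, end-cast and alternate cast events, with only the primary cast implemented here.
; CastSpell traces a short distance from the caster's first-person camera along its view, ignoring the caster.
; On a hit, the spell moves to the caster's casting point and rotates toward the impact, so it aims where the camera looks.
; Otherwise it takes the casting point's transform.
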(event Custom|CastSpell
  (bind _self self)
  (bind _casterpawn (Variables|Default|GetCasterPawn))
  (bind _casterpawn_2 (Variables|Default|GetCasterPawn))
  (bind _firstpersoncamera (Variables|/Game/Blueprints/BasePlayerPawn_BP.BasePlayerPawn_BP_C|GetFirstPersonCamera _casterpawn_2))
  (bind _spellcastingpoint (Variables|/Game/Blueprints/BasePlayerPawn_BP.BasePlayerPawn_BP_C|GetSpellCastingPoint _casterpawn))
  (bind _returnvalue (Transformation|GetWorldLocation _spellcastingpoint))
  (bind _returnvalue_2 (Transformation|GetWorldLocation _firstpersoncamera))
  (bind (_outhit _returnvalue_3) (Collision|LineTraceForObjects _returnvalue_2 (+ _returnvalue_2 (* (Math|Vector|GetForwardVector (Transformation|GetWorldRotation _firstpersoncamera)) 8e+02)) (Variables|Default|GetNewVar_0) false (Utilities|Array|MakeArray _casterpawn_2) "None"))
  (if _returnvalue_3
    (Transformation|SetActorTransform _self (Math|Transform|MakeTransform _returnvalue (Math|Rotator|FindLookatRotation _returnvalue (.ImpactPoint (Collision|BreakHitResult _outhit)))))
    (else
      (Transformation|SetActorTransform _self (Transformation|GetWorldTransform _spellcastingpoint)))))

(event Custom|AltCastSpell)

(event Custom|EndCastSpell)

(event Custom|AltEndCastSpell)

(event EventBeginPlay)

(fn ConstructionScript)