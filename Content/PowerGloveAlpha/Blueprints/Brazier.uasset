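; Brazier is a puzzle actor that spell projectiles light or extinguish by hitting it.
; A hit with element type 0 activates the fire effect and point light and sets IsLit, while type 2 turns them off and clears it.
; After either change and a short delay, it checks the referenced Door's CanPass flag and prints a hint on whether the door will open.
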(event Collision|EventHit
  (params (MyComp :type Primitive%20Component%20Object%20Reference) (Other :type Actor%20Object%20Reference) (OtherComp :type Primitive%20Component%20Object%20Reference) (bSelfMoved :type Boolean) (HitLocation :type Vector :default "0, 0, 0") (HitNormal :type Vector :default "0, 0, 0") (NormalImpulse :type Vector :default "0, 0, 0") (Hit :type Hit%20Result%20Structure%20%28by%20ref%29))
  (bind _pointlight (Variables|Default|GetPointLight))
  (bind _fire (Variables|Default|GetFire))
  (bind _asspell_projectile (Utilities|Casting|CastToSpellProjectile Other))
  (if (== (Variables|/Game/PowerGloveAlpha/Blueprints/SpellProjectile.SpellProjectile_C|GetElementType _asspell_projectile) 0)
    (Components|Activation|Activate _fire false)
    (Rendering|SetVisibility _pointlight true false)
    (Variables|Default|SetIsLit true)
    (Utilities|FlowControl|Delay 0.2 :!label _label)
    (if (Variables|/Game/PowerGloveAlpha/Blueprints/Door_Object_Version_2_Blueprint.Door_Object_Version_2_Blueprint_C|GetCanPass (Variables|Default|GetDoor))
      (Development|PrintString "The door seems to positively humm, 
lets see if you can go through" true true "(R=0.810000,G=0.000000,B=0.000000,A=1.000000)")
      (else
        (Development|PrintString "The door does not look impressed" true true "(R=0.760000,G=0.000000,B=0.000000,A=1.000000)")))
    (elif (== (Variables|/Game/PowerGloveAlpha/Blueprints/SpellProjectile.SpellProjectile_C|GetElementType _asspell_projectile) 2)
      (Components|Activation|Deactivate _fire)
      (Rendering|SetVisibility _pointlight false false)
      (Variables|Default|SetIsLit false)
      (goto _label))))

(fn ConstructionScript)