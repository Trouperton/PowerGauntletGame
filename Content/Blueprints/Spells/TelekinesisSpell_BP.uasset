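; Telekinesis spell that lets the caster pick up a carryable object in front of them and hold it.
; CastSpell line-traces from the first-person camera for a Pickable carryable mesh actor, disables its physics, ignores Pawn collision and snaps it to the caster's HoldingPoint.
; AltEndCastSpell detaches the held object, re-enables physics and clears the reference, leaving Pawn collision set to Ignore.
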(event EventAltEndCastSpell
  (|CallParentFunction)
  (if (Utilities|IsValid (Variables|Default|GetObjectHeld))
    (Transformation|DetachFromActor (Variables|Default|GetObjectHeld) "KeepRelative" "KeepRelative" "KeepRelative")
    (Collision|SetCollisionResponsetoChannel (Variables|/Script/Engine.StaticMeshActor|GetStaticMeshComponent (Variables|Default|GetObjectHeld)) "ECC_Pawn" "ECR_Ignore")
    (Physics|SetSimulatePhysics (Variables|/Script/Engine.StaticMeshActor|GetStaticMeshComponent (Variables|Default|GetObjectHeld)) true)
    (Variables|Default|SetObjectHeld 0)))

(event EventCastSpell
  (bind _casterpawn (Variables|Default|GetCasterPawn))
  (bind _firstpersoncamera (Variables|/Game/Blueprints/BasePlayerPawn_BP.BasePlayerPawn_BP_C|GetFirstPersonCamera _casterpawn))
  (bind _returnvalue (Transformation|GetWorldLocation _firstpersoncamera))
  (|CallParentFunction)
  (bind _outhit (Collision|LineTraceForObjects _returnvalue (+ _returnvalue (* (Math|Vector|GetForwardVector (Transformation|GetWorldRotation _firstpersoncamera)) 8e+02)) (Variables|Default|GetPickable) false (Utilities|Array|MakeArray _casterpawn) "None"))
  (bind _asbase_carryable_static_mesh_actor_bp (Utilities|Casting|CastToBaseCarryableStaticMeshActor_BP (.HitActor (Collision|BreakHitResult _outhit))))
  (bind _output_get (Variables|Default|SetObjectHeld _asbase_carryable_static_mesh_actor_bp))
  (Physics|SetSimulatePhysics (Variables|/Script/Engine.StaticMeshActor|GetStaticMeshComponent _output_get) false)
  (Collision|SetCollisionResponsetoChannel (Variables|/Script/Engine.StaticMeshActor|GetStaticMeshComponent _output_get) "ECC_Pawn" "ECR_Ignore")
  (Transformation|AttachComponentToComponent _asbase_carryable_static_mesh_actor_bp (Variables|/Game/Blueprints/BasePlayerPawn_BP.BasePlayerPawn_BP_C|GetHoldingPoint (Variables|Default|GetCasterPawn)) "None" "SnapToTarget" "KeepWorld" "KeepWorld" false))

(fn ConstructionScript
  (|CallParentFunction))