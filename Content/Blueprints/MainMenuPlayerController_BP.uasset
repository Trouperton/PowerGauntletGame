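; Main menu player controller that shows a production splash before opening the main menu.
; On BeginPlay it creates and stores both the production and main menu widgets, then adds the production widget to the viewport.
; After a short fixed delay it removes all widgets, adds the main menu and enables the mouse cursor.
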(event EventBeginPlay
  (bind _self self)
  (bind _returnvalue (UserInterface|CreateWidget "/Game/Blueprints/Widgets/ProductionWidget_BP.ProductionWidget_BP_C" _self))
  (Variables|Default|SetProductionWidget _returnvalue)
  (bind _returnvalue_2 (UserInterface|CreateWidget "/Game/Blueprints/Widgets/MainMenuWidget_BP.MainMenuWidget_BP_C" _self))
  (Variables|Default|SetMainMenuWidget _returnvalue_2)
  (UserInterface|Viewport|AddtoViewport (Variables|Default|GetProductionWidget) 0)
  (Utilities|FlowControl|Delay 3.0)
  (Viewport|RemoveAllWidgets)
  (UserInterface|Viewport|AddtoViewport (Variables|Default|GetMainMenuWidget) 0)
  (Variables|Default|SetbShowMouseCursor true))

(fn ConstructionScript)