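; Firebolt spell projectile Blueprint, a child that extends its parent's impact behavior.
; On impact it runs the parent ImpactScript, destroys its sphere collider, and swaps the fire particle system to an ending effect template.
; The actor destroys itself when the fire particle system finishes, letting the ending effect play out first.
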(event OnSystemFinished(FireParticleSystem)
  (params (PSystem :type Particle%20System%20Component%20Object%20Reference))
  (Actor|DestroyActor))

(event EventBeginPlay
  (|CallParentFunction) ; This node is disabled and will not be called.\nDrag off pins to build functionality.
)

(event Collision|EventActorBeginOverlap
  (params (OtherActor :type Actor%20Object%20Reference))
  (|CallParentFunction OtherActor) ; This node is disabled and will not be called.\nDrag off pins to build functionality.
)

(event EventTick
  (params (DeltaSeconds :type Float%20%28single-precision%29))
  (|CallParentFunction DeltaSeconds) ; This node is disabled and will not be called.\nDrag off pins to build functionality.
)

(fn ConstructionScript
  (|CallParentFunction))

(fn ImpactScript
  (|CallParentFunction)
  (Components|DestroyComponent (Variables|Default|GetSphereCollider))
  (Effects|Components|ParticleSystem|SetTemplate (Variables|Default|GetFireParticleSystem) (Variables|Default|GetEndingParticleSystem)))