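; Puzzle door actor that acts as a game exit, gated by the state of three braziers.
; Every Tick it sets CanPass true only when BrazierThree is lit and BrazierOne and BrazierTwo are unlit.
; When MainCharacter hits the door while CanPass is true, the game quits.
; Two flavor-text PrintString nodes about the door's reaction are left disconnected and never run.
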(event EventTick
  (params (DeltaSeconds :type Float%20%28single-precision%29))
  (if (not (Variables|/Game/PowerGloveAlpha/Blueprints/Brazier.Brazier_C|GetIsLit (Variables|Default|GetBrazierOne)))
    (if (not (Variables|/Game/PowerGloveAlpha/Blueprints/Brazier.Brazier_C|GetIsLit (Variables|Default|GetBrazierTwo)))
      (if (Variables|/Game/PowerGloveAlpha/Blueprints/Brazier.Brazier_C|GetIsLit (Variables|Default|GetBrazierThree))
        (Variables|Default|SetCanPass true)
        (else
          (Variables|Default|SetCanPass false :!label _label)))
      (else
        (goto _label)))
    (else
      (goto _label))))

(event Collision|EventHit
  (params (MyComp :type Primitive%20Component%20Object%20Reference) (Other :type Actor%20Object%20Reference) (OtherComp :type Primitive%20Component%20Object%20Reference) (bSelfMoved :type Boolean) (HitLocation :type Vector :default "0, 0, 0") (HitNormal :type Vector :default "0, 0, 0") (NormalImpulse :type Vector :default "0, 0, 0") (Hit :type Hit%20Result%20Structure%20%28by%20ref%29))
  (Utilities|Casting|CastToMainCharacter Other)
  (if (Variables|Default|GetCanPass)
    (Game|QuitGame (Game|GetPlayerController 0) "Quit" false)))

(fn ConstructionScript)