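; MainCharacter is the first-person player character for a spell-casting game with a brazier pattern puzzle, announced on screen at BeginPlay.
; Input axes and actions drive movement, camera look and jumping.
; NextSpell cycles a byte index through SpellList with wraparound, but Fire always casts FireBoltSpell on itself, ignoring that selection.
; Debug prints show the selected index, the capsule's forward vector every tick and optional construction.
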(event EventBeginPlay
  (Development|PrintString "Light the braziers in the correct pattern" true true "(R=0.930000,G=0.000000,B=0.000000,A=1.000000)" 2e+01))

(event EventTick
  (params (DeltaSeconds :type Float%20%28single-precision%29))
  (Development|PrintString (Utilities|String|ToString(Vector) (Math|Vector|GetForwardVector (Variables|Collision|GetCapsuleComponent)))))

(event Input|ActionEvents|InputActionJump
  (params (Key :type Key%20Structure :default "None"))
  ;[1 1 1] Movement controls.
  ;;[1 1 1] Handles jumping.
  (:Pressed
    (Character|Jump))
  (:Released
    (Character|StopJumping)))

(event Input|ActionEvents|InputActionFire
  (params (Key :type Key%20Structure :default "None"))
  (:Pressed
    (Default|CastSpell (Variables|Default|GetFireBoltSpell) self)))

(event Input|AxisEvents|InputAxisMoveForward
  (params (AxisValue :type Float%20%28single-precision%29))
  ;[1 1 1] Movement controls.
  ;;[1 1 1] Handles moving forward and backwards.
  (Pawn|Input|AddMovementInput (Transformation|GetActorForwardVector) AxisValue false))

(event Input|AxisEvents|InputAxisTurn
  (params (AxisValue :type Float%20%28single-precision%29))
  ;[1 1 1] Camera controls.
  (Pawn|Input|AddControllerYawInput AxisValue))

(event Input|AxisEvents|InputAxisLookUp
  (params (AxisValue :type Float%20%28single-precision%29))
  ;[1 1 1] Camera controls.
  (Pawn|Input|AddControllerPitchInput AxisValue))

(event Input|AxisEvents|InputAxisStrafeRight
  (params (AxisValue :type Float%20%28single-precision%29))
  ;[1 1 1] Movement controls.
  ;;[1 1 1] Handles moving left and right.
  (Pawn|Input|AddMovementInput (Transformation|GetActorRightVector) AxisValue false))

(event Input|AxisEvents|InputAxisNextSpell
  (params (AxisValue :type Float%20%28single-precision%29))
  (bind _spelllist (Variables|Default|GetSpellList))
  (bind _returnvalue (Utilities|Array|Length _spelllist))
  (bind _returnvalue_2 (Math|Conversions|ToByte(Integer) _returnvalue))
  ;[1 1 1] Checks if axis value is not equal to 0.
  (if (!= AxisValue 0.0)
    ;[1 1 1] Checks if current spell value plus the axis value is greater than or equal to the number of values stored in the Spell List
    (if (>= (+ (Variables|Default|GetCurrentSpell) (Math|Conversions|ToByte(Integer) (Math|Float|Truncate AxisValue))) _returnvalue_2)
      (if (< AxisValue 0.0)
        (Variables|Default|SetCurrentSpell (- _returnvalue_2 1))
        (else
          (Variables|Default|SetCurrentSpell 0)))
      (else
        (Variables|Default|SetCurrentSpell (+ (Variables|Default|GetCurrentSpell) (Math|Conversions|ToByte(Integer) (Math|Float|Truncate AxisValue))))))
    (Development|PrintString (Utilities|String|ToString(Byte) (Variables|Default|GetCurrentSpell)))))

(fn ConstructionScript
  (if (Variables|Default|GetDebugging)
    (Development|PrintString "MainCharacter created.")))