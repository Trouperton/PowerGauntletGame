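; SolvedChecker_BP_Child is a puzzle checker that removes a door once the puzzle's solution is met.
; Its CheckifSolved event compares each Solution entry to the ConditionsChecked entry at the same index, clearing the Solved flag on any mismatch.
; If every entry matches, it destroys the Door actor.
; The default event nodes are disabled, and the construction script only calls the parent.
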(event EventBeginPlay
  (|CallParentFunction) ; This node is disabled and will not be called.\nDrag off pins to build functionality.
)

(event Collision|EventActorBeginOverlap
  (params (OtherActor :type Actor%20Object%20Reference))
  (|CallParentFunction OtherActor) ; This node is disabled and will not be called.\nDrag off pins to build functionality.
)

(event EventTick
  (params (DeltaSeconds :type Float%20%28single-precision%29))
  (|CallParentFunction DeltaSeconds) ; This node is disabled and will not be called.\nDrag off pins to build functionality.
)

(event EventCheckifSolved
  (Variables|Default|SetSolved true)
  (for (_array_element _array_index) (Variables|Default|GetSolution)
    (if (not (Math|Boolean|Equal(Boolean) _array_element (Utilities|Array|Get(acopy) (Variables|Default|GetConditionsChecked) _array_index)))
      (Variables|Default|SetSolved false)))
  (if (Variables|Default|GetSolved)
    (Actor|DestroyActor (Variables|Default|GetDoor))))

(fn ConstructionScript
  (|CallParentFunction))