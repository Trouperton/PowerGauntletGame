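; PuzzleBrazier_BP is a brazier that serves as one condition in a multi-part puzzle.
; On BeginPlay and on every Hit, it runs the parent logic, then writes IsLit into the SolutionChecker's ConditionsChecked array at its SolutionPosition.
; After each write it asks the SolutionChecker to check whether the puzzle is solved.
; The graph never changes IsLit itself, only reports it.
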(event EventBeginPlay
  (bind _solutionchecker (Variables|Default|GetSolutionChecker))
  (|CallParentFunction)
  (Utilities|Array|SetArrayElem (Variables|/Game/Blueprints/SolvedChecker_BP.SolvedChecker_BP_C|GetConditionsChecked _solutionchecker) (Variables|Default|GetSolutionPosition) (Variables|Default|GetIsLit))
  (Default|CheckifSolved _solutionchecker))

(event Collision|EventActorBeginOverlap
  (params (OtherActor :type Actor%20Object%20Reference))
  (|CallParentFunction OtherActor) ; This node is disabled and will not be called.\nDrag off pins to build functionality.
)

(event EventTick
  (params (DeltaSeconds :type Float%20%28single-precision%29))
  (|CallParentFunction DeltaSeconds) ; This node is disabled and will not be called.\nDrag off pins to build functionality.
)

(event Collision|EventHit
  (params (MyComp :type Primitive%20Component%20Object%20Reference) (Other :type Actor%20Object%20Reference) (OtherComp :type Primitive%20Component%20Object%20Reference) (bSelfMoved :type Boolean) (HitLocation :type Vector :default "0, 0, 0") (HitNormal :type Vector :default "0, 0, 0") (NormalImpulse :type Vector :default "0, 0, 0") (Hit :type Hit%20Result%20Structure%20%28by%20ref%29))
  (bind _solutionchecker (Variables|Default|GetSolutionChecker))
  (|CallParentFunction MyComp Other OtherComp bSelfMoved HitLocation HitNormal NormalImpulse Hit)
  (Utilities|Array|SetArrayElem (Variables|/Game/Blueprints/SolvedChecker_BP.SolvedChecker_BP_C|GetConditionsChecked _solutionchecker) (Variables|Default|GetSolutionPosition) (Variables|Default|GetIsLit))
  (Default|CheckifSolved _solutionchecker))

(fn ConstructionScript
  (|CallParentFunction))