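; SolvedChecker_BP is an actor that checks whether the puzzle is solved and ends the game when it is.
; Its CheckIfSolved event compares the Solution array element by element with ConditionsChecked, and any mismatch marks it unsolved.
; On a full match it removes all widgets, shows EndScreenWidget_BP, waits briefly and quits the game.
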(event Custom|CheckIfSolved
  (Variables|Default|SetSolved true)
  (for (_array_element _array_index) (Variables|Default|GetSolution)
    (if (not (Math|Boolean|Equal(Boolean) _array_element (Utilities|Array|Get(acopy) (Variables|Default|GetConditionsChecked) _array_index)))
      (Variables|Default|SetSolved false)))
  (if (Variables|Default|GetSolved)
    (Viewport|RemoveAllWidgets)
    (bind _returnvalue (UserInterface|CreateWidget "/Game/Blueprints/Widgets/EndScreenWidget_BP.EndScreenWidget_BP_C" (Game|GetPlayerController 0)))
    (UserInterface|Viewport|AddtoViewport _returnvalue 0)
    (Utilities|FlowControl|Delay 3.0)
    (Game|QuitGame 0 "Quit" false)))

(event EventBeginPlay)

(event Collision|EventActorBeginOverlap
  (params (OtherActor :type Actor%20Object%20Reference)))

(event EventTick
  (params (DeltaSeconds :type Float%20%28single-precision%29)))

(fn ConstructionScript)