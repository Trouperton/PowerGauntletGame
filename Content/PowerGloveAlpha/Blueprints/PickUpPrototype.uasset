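; PickUpPrototype is an unfinished prototype actor, apparently meant to be carried in front of the player.
; On BeginPlay it finds the BasePlayerPawn_BP actor and caches it as CharacterToFollow.
; Disconnected SetActorLocation and Teleport nodes would place it a short distance along the player's first-person camera forward vector.
; Tick and overlap events are empty, so the actor never moves as written.
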(event EventBeginPlay
  (bind _returnvalue (Actor|GetActorOfClass "/Game/Blueprints/BasePlayerPawn_BP.BasePlayerPawn_BP_C"))
  (Variables|Default|SetCharacterToFollow _returnvalue))

(event Collision|EventActorBeginOverlap
  (params (OtherActor :type Actor%20Object%20Reference)))

(event EventTick
  (params (DeltaSeconds :type Float%20%28single-precision%29)))

(fn ConstructionScript)